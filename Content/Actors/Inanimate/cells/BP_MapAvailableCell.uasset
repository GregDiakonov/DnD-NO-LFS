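; Clickable grid cell marking a position on the map that the hero can move to.
; Hovering replaces any existing BP_MapSelectedCell with one spawned through BP_MapGrid at this cell's coordinates.
; Clicking spawns a selected cell there, asks DNDGameMode to move the hero to those coordinates, then destroys this cell.
; Older code that rotated and teleported KnightHero, including the GetRotationAngle helper, remains but never runs.
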(event `self.ReceiveActorOnClicked`
  (params (ButtonPressed :type "Key Structure"))
  (bind _coordinates (`self.Coordinates`))
  ;[1 1 1] Событие нажатия на ячейку
  (bind _returnvalue (`GameplayStatics.GetActorOfClass` "/Game/Actors/Inanimate/grids/BP_MapGrid.BP_MapGrid_C"))
  (`/Game/Actors/Inanimate/grids/BP_MapGrid.SpawnActorOnCell` :`self` _returnvalue :`Actor` "/Game/Actors/Inanimate/cells/BP_MapSelectedCell.BP_MapSelectedCell_C" :`Coordinates` _coordinates)
  (bind _asdndgame_mode (cast `/Game/GameModes/DNDGameMode` (`GameplayStatics.GetGameMode`)))
  (`/Game/GameModes/DNDGameMode.MoveHeroToPositionOnMap` _asdndgame_mode _coordinates)
  (`self.K2_DestroyActor`))

(event `self.ReceiveActorBeginCursorOver`
  (bind _coordinates (`self.Coordinates`))
  ;[1 1 1] События начала наведения курсора на ячейку
  (bind _returnvalue (`GameplayStatics.GetActorOfClass` "/Game/Actors/Inanimate/cells/BP_MapSelectedCell.BP_MapSelectedCell_C"))
  (if (`KismetSystemLibrary.IsValid` _returnvalue)
    (`self.K2_DestroyActor` _returnvalue))
  (bind _returnvalue_2 (`GameplayStatics.GetActorOfClass` "/Game/Actors/Inanimate/grids/BP_MapGrid.BP_MapGrid_C"))
  (bind _spawnedactor (`/Game/Actors/Inanimate/grids/BP_MapGrid.SpawnActorOnCell` :`self` _returnvalue_2 :`Actor` "/Game/Actors/Inanimate/cells/BP_MapSelectedCell.BP_MapSelectedCell_C" :`Coordinates` _coordinates))
  (bind _asbp_map_selected_cell (cast `/Game/Actors/Inanimate/cells/BP_MapSelectedCell` _spawnedactor))
  (set `/Game/Actors/Inanimate/cells/BP_MapSelectedCell.Coordinates` _coordinates _asbp_map_selected_cell))

(event `self.ReceiveActorEndCursorOver`
  ;[1 1 1] Событие конца наведения курсора на ячейку
)

(fn `Get Rotation Angle`
  (params (VectorFrom :type "Vector2D Structure") (VectorTo :type "Vector2D Structure"))
  (returns (DegreeAngle :type "Float (double-precision)"))
  (bind _returnvalue (`KismetMathLibrary.SignOfFloat` (`KismetMathLibrary.CrossProduct2D` VectorFrom VectorTo)))
  (bind _returnvalue_2 (`KismetMathLibrary.RadiansToDegrees` (`KismetMathLibrary.Acos` (/ (`KismetMathLibrary.DotProduct2D` VectorFrom VectorTo) (* (`KismetMathLibrary.VSize2D` VectorFrom) (`KismetMathLibrary.VSize2D` VectorTo))))))
  ;[0.25 0.25 0.25] Получение угла поворота (не используется)
  (if (and (== _returnvalue 0.0) (!= _returnvalue_2 0.0))
    (return 180.0)
    (else
      (return (* _returnvalue_2 _returnvalue)))))

(fn `UserConstructionScript`)