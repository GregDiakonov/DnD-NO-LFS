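; BP_MapStartFightCell is a map grid cell that shows a fight-start selection marker while the cursor hovers over it.
; On hover it has BP_MapGrid spawn a BP_MapSelectStartFightCell at its coordinates, passes along coordinates and enemy position, and lifts it slightly.
; When hover ends, a short delay precedes destroying the first selection cell found in the world.
; The click event is empty, and the hero-move call is unconnected.
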(event `self.ReceiveBeginPlay`)

(event `self.ReceiveActorOnClicked`
  (params (ButtonPressed :type "Key Structure")))

(event `self.ReceiveActorBeginCursorOver`
  (bind _coordinates (`self.Coordinates`))
  ;[1 1 1] Событие начала наведения курсора на ячейку
  (bind _returnvalue (`GameplayStatics.GetActorOfClass` "/Game/Actors/Inanimate/grids/BP_MapGrid.BP_MapGrid_C"))
  (bind _spawnedactor (`/Game/Actors/Inanimate/grids/BP_MapGrid.SpawnActorOnCell` :`self` _returnvalue :`Actor` "/Game/Actors/Inanimate/cells/BP_MapSelectStartFightCell.BP_MapSelectStartFightCell_C" :`Coordinates` _coordinates))
  (bind _asbp_map_select_start_fight_cell (cast `/Game/Actors/Inanimate/cells/BP_MapSelectStartFightCell` _spawnedactor))
  (set `/Game/Actors/Inanimate/cells/BP_MapSelectStartFightCell.Coordinates` _coordinates _asbp_map_select_start_fight_cell)
  (set `/Game/Actors/Inanimate/cells/BP_MapSelectStartFightCell.EnemyPosition` (`self.EnemyPosistion`) _asbp_map_select_start_fight_cell)
  (bind (_returnvalue_x _returnvalue_y _returnvalue_z) (`KismetMathLibrary.BreakVector` (`self.K2_GetActorLocation` _asbp_map_select_start_fight_cell)))
  (`self.K2_SetActorLocation` _asbp_map_select_start_fight_cell (`KismetMathLibrary.MakeVector` _returnvalue_x _returnvalue_y (+ _returnvalue_z 2.0)) false false))

(event `self.ReceiveActorEndCursorOver`
  ;[1 1 1] Событие конца наведения курсора на ячейку
  (`KismetSystemLibrary.Delay` 0.2)
  (bind _returnvalue (`GameplayStatics.GetActorOfClass` "/Game/Actors/Inanimate/cells/BP_MapSelectStartFightCell.BP_MapSelectStartFightCell_C"))
  (`self.K2_DestroyActor` _returnvalue))

(fn `UserConstructionScript`)