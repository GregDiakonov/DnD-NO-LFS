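; BP_MapSelectedCell is a clickable map cell actor that sends the hero to its position.
; On click it casts the game mode to DNDGameMode and calls MoveHeroToPositionOnMap with its Coordinates.
; A GetRotationAngle helper computes the signed angle in degrees between two 2D vectors, returning 180 for opposite ones, but nothing in this Blueprint calls it.
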(event `self.ReceiveBeginPlay`)

(event `self.ReceiveActorOnClicked`
  (params (ButtonPressed :type "Key Structure"))
  ;[1 1 1] События нажатия на ячейку
  (bind _asdndgame_mode (cast `/Game/GameModes/DNDGameMode` (`GameplayStatics.GetGameMode`)))
  (`/Game/GameModes/DNDGameMode.MoveHeroToPositionOnMap` _asdndgame_mode (`self.Coordinates`)))

(event `self.ReceiveActorEndCursorOver`)

(fn `Get Rotation Angle`
  (params (VectorFrom :type "Vector2D Structure") (VectorTo :type "Vector2D Structure"))
  (returns (DegreeAngle :type "Float (double-precision)"))
  (bind _returnvalue (`KismetMathLibrary.SignOfFloat` (`KismetMathLibrary.CrossProduct2D` VectorFrom VectorTo)))
  (bind _returnvalue_2 (`KismetMathLibrary.RadiansToDegrees` (`KismetMathLibrary.Acos` (/ (`KismetMathLibrary.DotProduct2D` VectorFrom VectorTo) (* (`KismetMathLibrary.VSize2D` VectorFrom) (`KismetMathLibrary.VSize2D` VectorTo))))))
  (if (and (== _returnvalue 0.0) (!= _returnvalue_2 0.0))
    (return 180.0)
    (else
      (return (* _returnvalue_2 _returnvalue)))))

(fn `UserConstructionScript`)