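; BP_MapGrid is the map grid actor that builds a Length by Width field of cells and provides cell-based placement.
; BeginPlay spawns BP_MapCellLocation actors at CellDistance spacing, assigns center-relative coordinates and stores CenterLocation.
; TransformToAbsoluteCoordinates converts coordinates to world XY, negating X unlike the spawn loop, for camera moves, actor teleports and bounds-checked spawning.
; GetNearCells returns a square block of coordinates around Center, without bounds checks.
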(event `self.ReceiveBeginPlay`
  (bind (_returnvalue_x _returnvalue_y _returnvalue_z) (`KismetMathLibrary.BreakVector` (`self.K2_GetActorLocation`)))
  (bind _celldistance (`self.CellDistance`))
  (bind _celldistance_2 (`self.CellDistance`))
  ;[1 1 1] При создании карты
  (for _index (range (`self.Length`))
    (for _index_2 (range (`self.Width`))
      (`|SpawnActorFromClass` "/Game/Actors/Inanimate/cells/BP_MapCellLocation.BP_MapCellLocation_C" (`KismetMathLibrary.MakeTransform` (`KismetMathLibrary.MakeVector` (+ (* _celldistance _index) _returnvalue_x) (+ (* _celldistance _index_2) _returnvalue_y) _returnvalue_z)) "Undefined" "MultiplyWithRoot" null (make `/Game/Actors/Inanimate/grids/ST_MapCoordinates` (- _index (/ (`self.Length`) 2)) (- _index_2 (/ (`self.Width`) 2))) null)
      (set `self.CenterLocation` (+ (`KismetMathLibrary.MakeVector` (* (/ (`self.Length`) 2) _celldistance_2) (* (/ (`self.Width`) 2) _celldistance_2)) (`self.K2_GetActorLocation`))))))

(event `MoveCameraToCell`
  (params (Coordinates :type "/Game/Actors/Inanimate/grids/ST_MapCoordinates Structure"))
  ;[1 1 1] Перенос камеры на заданную ячейку
  (bind _returnvalue (`GameplayStatics.GetActorOfClass` "/Script/Engine.CameraActor"))
  (bind (_absolutex _absolutey) (`self.TransformToAbsoluteCoordinates` Coordinates))
  (`self.K2_SetActorLocation` _returnvalue (`KismetMathLibrary.MakeVector` _absolutex (+ _absolutey -1000.0) 1000.0) false false))

(event `MoveActorToCell`
  (params (Actor :type "Actor Object Reference") (Cell :type "/Game/Actors/Inanimate/grids/ST_MapCoordinates Structure"))
  ;[1 1 1] Перенос актора на заданную ячейку
  (bind (_absolutex _absolutey) (`self.TransformToAbsoluteCoordinates` Cell))
  (`self.K2_TeleportTo` Actor (`KismetMathLibrary.MakeVector` _absolutex _absolutey) (`self.K2_GetActorRotation` Actor)))

(fn `GetNearCells`
  (params (Center :type "/Game/Actors/Inanimate/grids/ST_MapCoordinates Structure") (Radius :type Integer))
  (returns (NearCells :type "Array of /Game/Actors/Inanimate/grids/ST_MapCoordinates Structure"))
  (locals (Cells :type "Array of /Game/Actors/Inanimate/grids/ST_MapCoordinates Structure"))
  (bind _returnvalue (- Radius 1))
  (bind _cells (`local.Cells`))
  ;[1 1 1] Получение координат ячеек, ближайших к заданной
  (for _index (range (- Center_X_3_7C507CE37649539D82039986B43EC08E _returnvalue) (+ (+ Center_X_3_7C507CE37649539D82039986B43EC08E _returnvalue) 1))
    (for _index_2 (range (- Center_Y_5_AD22050736425D4D478D70B67B24B40B _returnvalue) (+ (+ Center_Y_5_AD22050736425D4D478D70B67B24B40B _returnvalue) 1))
      (`KismetArrayLibrary.Array_Add` _cells (make `/Game/Actors/Inanimate/grids/ST_MapCoordinates` _index _index_2))))
  (return _cells))

(fn `SpawnActorOnCell`
  (params (Actor :type "Actor Class Reference") (Coordinates :type "/Game/Actors/Inanimate/grids/ST_MapCoordinates Structure") (Scale :type "Vector Structure" :default (1.0 1.0 1.0)) (Rotation :type "Rotator Structure"))
  (returns (SpawnedActor :type "Actor Object Reference"))
  (locals (NullActor :type "Actor Object Reference"))
  (bind (_x _y) (break `/Game/Actors/Inanimate/grids/ST_MapCoordinates` Coordinates))
  (bind _returnvalue (/ (`self.Width`) 2))
  (bind _returnvalue_2 (/ (`self.Length`) 2))
  ;[1 1 1] Создание актора на заданной ячейке
  (if (and (`KismetMathLibrary.InRange_IntInt` _x (- 0 _returnvalue_2) _returnvalue_2) (`KismetMathLibrary.InRange_IntInt` _y (- 0 _returnvalue) _returnvalue))
    (bind (_absolutex _absolutey) (`self.TransformToAbsoluteCoordinates` Coordinates))
    (bind _returnvalue_3 (`|SpawnActorFromClass` Actor (`KismetMathLibrary.MakeTransform` (`KismetMathLibrary.MakeVector` _absolutex _absolutey) Rotation Scale) "Undefined" "MultiplyWithRoot" null null))
    (return _returnvalue_3)
    (else
      (return (`local.NullActor`)))))

(fn `TransformToAbsoluteCoordinates`
  (params (Coordinates :type "/Game/Actors/Inanimate/grids/ST_MapCoordinates Structure"))
  (returns (AbsoluteX :type "Float (double-precision)") (AbsoluteY :type "Float (double-precision)"))
  (bind _celldistance (`self.CellDistance`))
  ;[1 1 1] Трансформирование координат на карте в абсолютные координаты мира
  (return (+ (* (* Coordinates_X_3_7C507CE37649539D82039986B43EC08E _celldistance) -1.0) (.x (`self.CenterLocation`))) (+ (* Coordinates_Y_5_AD22050736425D4D478D70B67B24B40B _celldistance) (.y (`self.CenterLocation`)))))

(fn `UserConstructionScript`)